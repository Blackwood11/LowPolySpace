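; BP_Cloud is a decorative cloud actor that drifts slowly across the level.
; Its construction script gives the Cloud mesh component a random mesh from five variants and a random uniform scale from six presets.
; On BeginPlay, a single MoveComponentTo slides the mesh to the EndLocation component's relative position over a random duration of several minutes, keeping its rotation, with no looping.
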(event `self.ReceiveBeginPlay`
  ;[1 1 1] Move cloud to end location
  (`KismetSystemLibrary.MoveComponentTo` (`self.Cloud`) (`SceneComponent.RelativeLocation` (`self.EndLocation`)) (`SceneComponent.RelativeRotation` (`self.Cloud`)) false false (`KismetMathLibrary.RandomFloatInRange` 300.0 500.0)))

(fn `UserConstructionScript`
  ;[1 1 1] Set a random cloud mesh on construction.
  (`StaticMeshComponent.SetStaticMesh` (`self.Cloud`) (select `int` (`KismetMathLibrary.RandomIntegerInRange` 0 4) :`0` "/Game/LowPolyUltimatePack/Meshes/nature/M_cloud01.M_cloud01" :`1` "/Game/LowPolyUltimatePack/Meshes/nature/M_cloud02.M_cloud02" :`2` "/Game/LowPolyUltimatePack/Meshes/nature/M_cloud03.M_cloud03" :`3` "/Game/LowPolyUltimatePack/Meshes/nature/M_cloud04.M_cloud04" :`4` "/Game/LowPolyUltimatePack/Meshes/nature/M_cloud05.M_cloud05" :!type "StaticMesh Object Reference"))
  ;[1 1 1] Set a random scale for the cloud that is being spawned
  (`SceneComponent.SetRelativeScale3D` (`self.Cloud`) (select `int` (`KismetMathLibrary.RandomIntegerInRange` 0 5) :`0` (2.0 2.0 2.0) :`1` (5.0 5.0 5.0) :`2` (8.0 8.0 8.0) :`3` (10.0 10.0 10.0) :`4` (15.0 15.0 15.0) :`5` (20.0 20.0 20.0) :!type "Vector Structure")))