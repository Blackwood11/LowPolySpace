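; LogWallBP is a procedural wall prop for Level 1, built from a row of static mesh logs.
; The Construction Script adds Length mesh components along local X, each with slightly randomized rotation and scale.
; Each offset is the index times a random step, so placement jitter grows along the row.
; The randomness is unseeded, so the layout changes on reconstruction, and the event graph has no active logic.
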(fn `UserConstructionScript`
  (for _index (range (`self.Length`))
    (`AddComponent|NODE_AddStaticMeshComponent-0` :`RelativeTransform` (`KismetMathLibrary.MakeTransform` (`KismetMathLibrary.MakeVector` (* _index (`KismetMathLibrary.RandomFloatInRange` 27.0 30.0))) (`KismetMathLibrary.MakeRotator` (`KismetMathLibrary.RandomFloatInRange` -3.0 3.0) (`KismetMathLibrary.RandomFloatInRange` -3.0 3.0) (`KismetMathLibrary.RandomFloatInRange` -3.0 3.0)) (`KismetMathLibrary.MakeVector` (`KismetMathLibrary.RandomFloatInRange` 1.2 1.5) (`KismetMathLibrary.RandomFloatInRange` 1.2 1.5) (`KismetMathLibrary.RandomFloatInRange` 1.0 1.6))))))