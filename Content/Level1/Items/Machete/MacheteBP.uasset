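; MacheteBP is the machete item actor for Level1.
; Shortly after BeginPlay, it checks whether its parent actor is the FirstPersonCharacter and turns mesh physics off if so, or on otherwise.
; A Disable function turns off both physics simulation and collision on the machete mesh.
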(event `self.ReceiveBeginPlay`
  (bind _machete (`self.Machete`))
  (`KismetSystemLibrary.Delay` 0.01)
  (if (== (`GameplayStatics.GetObjectClass` (`self.GetAttachParentActor`)) "/Game/Level1/Characters/FirstPersonCharacter.FirstPersonCharacter_C")
    (`PrimitiveComponent.SetSimulatePhysics` _machete false)
    (else
      (`PrimitiveComponent.SetSimulatePhysics` _machete true))))

(fn `Disable`
  (bind _machete (`self.Machete`))
  (`PrimitiveComponent.SetSimulatePhysics` _machete false)
  (`PrimitiveComponent.SetCollisionEnabled` _machete "NoCollision"))

(fn `UserConstructionScript`)